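; Blueprint function library with two static helpers for cursor/input mode and trace results.
; SetShowMouseCursor toggles the cursor on player controller 0, switching to UI-only input with a focused widget and no mouse lock when shown, or game-only input when hidden.
; GetHitLocation returns a hit's impact point, falling back to the trace end when nothing is hit.
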(fn SetShowMouseCursor
  (params (Show :type Boolean) (InWidgetToFocus :type Widget%20Object%20Reference))
  (bind _returnvalue (Game|GetPlayerController 0))
  (Utilities|IsValid _returnvalue
    (:Is%20Valid
      (Variables|/Script/Engine.PlayerController|SetbShowMouseCursor _returnvalue Show)
      (if Show
        (Input|SetInputModeUIOnly (Game|GetPlayerController 0) InWidgetToFocus "DoNotLock")
        (else
          (Input|SetInputModeGameOnly (Game|GetPlayerController 0)))))))

(fn GetHitLocation
  (params (Hit :type Hit%20Result%20Structure%20%28by%20ref%29) (bHit :type Boolean))
  (bind (_bblockinghit _binitialoverlap _time _distance _location _impactpoint _normal _impactnormal _physmat _hitactor _hitcomponent _hitbonename _hititem _elementindex _faceindex _tracestart _traceend) (Collision|BreakHitResult Hit))
  (if bHit
    (return _impactpoint)
    (else
      (return _traceend))))